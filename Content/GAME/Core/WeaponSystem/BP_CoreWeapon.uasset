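; Core weapon actor that equips itself to an overlapping BP_CoreCharacter and handles single, burst and automatic fire timed from RPM.
; StartFire shakes the camera and expands shotgun shots into pellets, each calling FinishFiring to spawn a projectile or apply hitscan damage, impulse and effects.
; ShootingMath orients shots from the muzzle toward the aim trace's hit point.
; Shotgun spread is either a random cone or screen-deprojected horizontal/vertical lines, mirrored halfway through the pellets.
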(event OnComponentBeginOverlap(Root)
  (params (OverlappedComponent :type Primitive%20Component%20Object%20Reference) (OtherActor :type Actor%20Object%20Reference) (OtherComp :type Primitive%20Component%20Object%20Reference) (OtherBodyIndex :type Integer) (bFromSweep :type Boolean) (SweepResult :type Hit%20Result%20Structure%20%28by%20ref%29))
  ;[1 1 1] If a player overlaps the weapon, equip it as a new weapon
  (bind _asbp_core_character (Utilities|Casting|CastToBP_CoreCharacter OtherActor))
  (Development|PrintString "Hello")
  (Variables|Refs|SetCharacterRef _asbp_core_character)
  (Default|EquipNewWeapon (Variables|Refs|GetCharacterRef) self (Variables|Stats|Generic|GetWeaponSlot)))

(event Custom|ResetBurstDelay
  ;[1 1 1] Burst fire and then wait for the next shot
  (Utilities|FlowControl|Delay (Variables|Internal|GetTimeBetweenShots))
  (Utilities|FlowControl|DoOnce false) ; enters at Reset
)

(event Custom|StartFire
  (if (Variables|Default|GetFireButtonHeld?) ; Check if the button is pressed in real time
    (Class|PlayerController|ClientPlayCameraShake (Game|GetPlayerController 0) "/Game/GAME/Core/WeaponSystem/CameraShake/BP_ShootShake.BP_ShootShake_C" (Variables|Stats|Generic|GetCameraShakeScale) "CameraLocal" "0, 0, 0")
    ;[1 1 1] If it's a shotgun, calculate how many pellets to fire, if there are less than two, don't add pellets
    (if (Variables|Stats|Shotgun|GetIsShotgun?)
      (if (<= (Variables|Stats|Shotgun|GetShotgunPellets) 1)
        (CallFunction|FinishFiring :!label _label)
        (else
          (|CalculateNumberOfPellets)))
      (else
        (goto _label)))))

(event Custom|Fire
  ;[1 1 1] Fire weapon based on firing mode
  (switch Utilities|FlowControl|Switch|SwitchonE_FireMode (Variables|Stats|Generic|GetEFireMode)
    (:NewEnumerator0
      ;[1 1 1] Fire once and wait for the next shot
      (Utilities|FlowControl|DoOnce false
        (:Completed
          (CallFunction|StartFire)
          (CallFunction|ResetSingleFireDelay))))
    (:NewEnumerator1
      ;[1 1 1] Burst fire and then wait for the next shot
      (Utilities|FlowControl|DoOnce false
        (:Completed
          (Utilities|BurstLoop (Variables|Default|GetBurstShots) (Variables|Internal|GetBurstTimeBetweenShots)
            (:then
              (CallFunction|StartFire)
              (CallFunction|ResetBurstDelay))))))
    (:NewEnumerator2
      (Utilities|FlowControl|Sequence
        (:then_0
          (Utilities|FlowControl|DoOnce false
            (:Completed
              (CallFunction|StartFire))))
        (:then_1
          (CallFunction|AutoFireStart))))))

(event Custom|FinishFiring
  ;[1 1 1] Finish firing based on weapon type
  (switch Utilities|FlowControl|Switch|SwitchonE_ProjectileType (Variables|Stats|Generic|GetE_ProjectileType)
    (:NewEnumerator0
      ;[1 1 1] Fire projectile
      (bind (_outhit _impactpointoutput _tracestartoutput _rotationoutput _currentmuzzlelocationoutput) (CallFunction|ShootingMath))
      (Utilities|FlowControl|Sequence
        (:then_0
          (Game|SpawnActorfromClass (Variables|Stats|Generic|GetProjectileClass) (Math|Transform|MakeTransform _currentmuzzlelocationoutput _rotationoutput "1,1,1") "AlwaysSpawn" 0 0))
        (:then_1
          (Audio|PlaySound2D (Variables|Cosmetic|Sounds|GetFiringSound) 1.0 1.0 0.0 0 0))))
    (:NewEnumerator1
      (bind _outhit_2 (CallFunction|ShootingMath))
      (Utilities|FlowControl|Sequence
        (:then_0
          ;[1 1 1] Apply damage
          (if (Variables|Stats|Shotgun|GetIsShotgun?)
            (if (.bBlockingHit (Collision|BreakHitResult _outhit_2)) ; Each pellet deals one damage
              (Game|Damage|ApplyDamage (.HitActor (Collision|BreakHitResult _outhit_2)) (Variables|Stats|Generic|GetHitScanDamage) (Game|GetPlayerController 0) (Variables|Refs|GetCharacterRef) "/Script/Engine.DamageType" :!label _label))
            (else
              (goto _label))))
        (:then_1
          ;[1 1 1] Apply physics to impact location
          (if (Variables|Stats|Shotgun|GetIsShotgun?)
            (Utilities|FlowControl|DoOnce false
              (:Completed
                _)))
          (Game|SpawnActorfromClass (Variables|Default|GetHitScanImpulse) (Math|Transform|MakeTransform (Variables|Internal|GetCurrentImpactPoint) "0, 0, 0" "1,1,1") "Undefined" 0 0))
        (:then_2
          ;[1 1 1] Effects
          (Effects|SpawnEmitterAttached (Variables|Cosmetic|Effects|GetFX_HitscanMuzzle) (Variables|Default|GetWeaponMesh) "" (Variables|Internal|GetCurrentMuzzleLocation) "0, 0, 0" "1.000000,1.000000,1.000000" "KeepWorldPosition")
          (bind _returnvalue (Effects|SpawnEmitteratLocation (Variables|Cosmetic|Effects|GetFX_HitscanTrail) (Variables|Internal|GetCurrentMuzzleLocation) (Variables|Internal|GetCurrentTraceRotation)))
          (Class|ParticleSystemComponent|SetBeamSourcePoint _returnvalue 0 (Variables|Internal|GetCurrentMuzzleLocation))
          (Class|ParticleSystemComponent|SetBeamTargetPoint _returnvalue 0 (Variables|Internal|GetCurrentImpactPoint))
          (Effects|SpawnEmitteratLocation (Variables|Cosmetic|Effects|GetFX_HitscanImpact) (Variables|Internal|GetCurrentImpactPoint)))
        (:then_3
          (Audio|PlaySound2D (Variables|Cosmetic|Sounds|GetFiringSound) 1.0 1.0 0.0 0 0)
          (Audio|PlaySoundatLocation "/Game/GAME/Assets/Audio/Weapon_AssaultRifle/Mono/AssaultRifle_ImpactConcrete_Cue.AssaultRifle_ImpactConcrete_Cue" (Variables|Internal|GetCurrentImpactPoint) "0, 0, 0" 1.0 1.0 0.0 0 0 0))))))

(event Custom|ResetSingleFireDelay
  ;[1 1 1] Fire once and wait for the next shot
  (Utilities|FlowControl|Delay (Variables|Internal|GetTimeBetweenShots))
  (Utilities|FlowControl|DoOnce false) ; enters at Reset
)

(event Custom|AutoFireStop
  ;[1 1 1] Stop auto fire if the timer has run out and the fire button isn't being held
  (Utilities|FlowControl|Delay (Utilities|Time|GetTimerRemainingTimebyHandle (Variables|Default|GetAutoFireTimerHandle)))
  (if (not (Variables|Default|GetFireButtonHeld?))
    (Utilities|FlowControl|Sequence
      (:then_0
        (Utilities|FlowControl|DoOnce false) ; enters at Reset
      )
      (:then_1
        (Utilities|Time|ClearandInvalidateTimerbyHandle (Variables|Default|GetAutoFireTimerHandle))))))

(event Custom|ResetShotgun
  ;[1 1 1] Apply physics to impact location
  (Utilities|FlowControl|Sequence
    (:then_0
      (Utilities|FlowControl|DoOnce false) ; enters at Reset
    )
    (:then_1
      (|G_ChangeShotgunFiringDirection))))

(event Custom|AutoFireStart
  ;[1 1 1] Start firing after each shot is rechambered and cache the timer handle to use elsewhere
  (bind _returnvalue (Utilities|Time|SetTimerbyEvent (delegate Custom|StartFire) (Variables|Internal|GetTimeBetweenShots) true))
  (Variables|Default|SetAutoFireTimerHandle _returnvalue))

(event Custom|FireButtonHeld
  (params (FireButtonHeld? :type Boolean))
  ;[1 1 1] Real time checking for if the fire button is held
  (Variables|Default|SetFireButtonHeld? FireButtonHeld?))

(event EventBeginPlay
  ;[1 1 1] Calculate fire rate
  (Variables|Internal|SetTimeBetweenShots (/ 6e+01 (Variables|Stats|Generic|GetRPM)))
  (Variables|Internal|SetBurstTimeBetweenShots (/ 6e+01 (Variables|Stats|Generic|GetBurstRPM))))

(fn ConstructionScript)

(fn SprayCone
  (params (InVec :type Vector) (A :type Float%20%28single-precision%29))
  (bind (_x _y _z) (Math|Vector|BreakVector InVec))
  (bind _returnvalue (* A 2e+02))
  (return (Math|Vector|MakeVector (+ _x (Math|Random|RandomFloatinRange (* _returnvalue -1.0) _returnvalue)) (+ _y (Math|Random|RandomFloatinRange (* _returnvalue -1.0) _returnvalue)) (+ _z (Math|Random|RandomFloatinRange (* _returnvalue -1.0) _returnvalue)))))

(fn ShootTrace
  (bind _returnvalue (Game|GetPlayerController 0))
  (bind _returnvalue_2 (Game|GetPlayerController 0))
  (bind _internalshotgunsprayoffset (Variables|Internal|GetInternalShotgunSprayOffset))
  (bind _shotgunsprayhalfwayswitch (Variables|Internal|GetShotgunSprayHalfwaySwitch))
  (bind _internalshotgunsprayoffset_2 (Variables|Internal|GetInternalShotgunSprayOffset))
  (bind _shotgunsprayhalfwayswitch_2 (Variables|Internal|GetShotgunSprayHalfwaySwitch))
  (bind (_sizex _sizey) (HUD|GetViewportSize _returnvalue))
  (bind (_sizex_2 _sizey_2) (HUD|GetViewportSize _returnvalue_2))
  (bind _returnvalue_3 (Math|Conversions|ToFloat(Integer) _sizex))
  (bind _returnvalue_4 (Math|Conversions|ToFloat(Integer) _sizey))
  (bind _returnvalue_5 (Math|Conversions|ToFloat(Integer) _sizex_2))
  (bind _returnvalue_6 (Math|Conversions|ToFloat(Integer) _sizey_2))
  (bind _returnvalue_7 (/ _returnvalue_3 2.0))
  (bind _returnvalue_8 (/ _returnvalue_4 2.0))
  (bind _returnvalue_9 (/ _returnvalue_5 2.0))
  (bind _returnvalue_10 (/ _returnvalue_6 2.0))
  (bind _returnvalue_11 (- _returnvalue_8 _internalshotgunsprayoffset))
  (bind _returnvalue_12 (- _returnvalue_9 _internalshotgunsprayoffset_2))
  (bind _returnvalue_13 (+ _returnvalue_9 _internalshotgunsprayoffset_2))
  (bind _returnvalue_14 (+ _returnvalue_8 _internalshotgunsprayoffset))
  (bind _returnvalue_15 (select _shotgunsprayhalfwayswitch _returnvalue_11 _returnvalue_14))
  (bind _returnvalue_16 (select _shotgunsprayhalfwayswitch_2 _returnvalue_12 _returnvalue_13))
  (bind (_worldlocation _worlddirection) (Class|PlayerController|DeprojectScreenPositiontoWorld _returnvalue _returnvalue_7 _returnvalue_15))
  (bind (_worldlocation_2 _worlddirection_2) (Class|PlayerController|DeprojectScreenPositiontoWorld _returnvalue_2 _returnvalue_16 _returnvalue_10))
  (switch Utilities|FlowControl|Switch|SwitchonE_ShotgunSprayType (Variables|Stats|Shotgun|GetShotgunSprayType)
    (:NewEnumerator0
      ;[1 1 1] Cone Spread
      (bind _characterref (Variables|Refs|GetCharacterRef)
        (:then
          (bind (_outhit _returnvalue_17) (Collision|LineTraceByChannel (Transformation|GetWorldLocation (Variables|/Game/GAME/Core/BP_CoreCharacter.BP_CoreCharacter_C|GetAimArrow _characterref)) (CallFunction|SprayCone (+ (Transformation|GetWorldLocation (Variables|/Game/GAME/Core/BP_CoreCharacter.BP_CoreCharacter_C|GetAimArrow _characterref)) (* (Math|Vector|GetForwardVector (Variables|/Game/GAME/Core/BP_CoreCharacter.BP_CoreCharacter_C|GetAimArrow _characterref)) 1e+04)) (select (Variables|Stats|Shotgun|GetIsShotgun?) (Variables|Stats|Shotgun|GetShotgunConeSize) 0.0)) "TraceTypeQuery1" false 0 "None"))
          (return (Variables|/Game/GAME/Core/BP_CoreCharacter.BP_CoreCharacter_C|GetAimArrow _characterref) _outhit _returnvalue_17))
        (:else)))
    (:NewEnumerator1
      (Variables|Refs|GetCharacterRef
        (:then
          (bind (_outhit_2 _returnvalue_18) (Collision|LineTraceByChannel _worldlocation_2 (+ _worldlocation_2 (* _worlddirection_2 3.5e+04)) "TraceTypeQuery1" false 0 "None"))
          (return (Variables|/Game/GAME/Core/BP_CoreCharacter.BP_CoreCharacter_C|GetAimArrow (Variables|Refs|GetCharacterRef)) _outhit_2 _returnvalue_18))
        (:else)))
    (:NewEnumerator2
      (Variables|Refs|GetCharacterRef
        (:then
          (bind (_outhit_3 _returnvalue_19) (Collision|LineTraceByChannel _worldlocation (+ _worldlocation (* _worlddirection 3.5e+04)) "TraceTypeQuery1" false 0 "None"))
          (return (Variables|/Game/GAME/Core/BP_CoreCharacter.BP_CoreCharacter_C|GetAimArrow (Variables|Refs|GetCharacterRef)) _outhit_3 _returnvalue_19))
        (:else)))))

(fn ShootingMath
  (bind _weaponmesh (Variables|Default|GetWeaponMesh))
  (bind _returnvalue (Transformation|GetSocketLocation _weaponmesh "Muzzle"))
  (Variables|Refs|GetCharacterRef
    (:then
      (bind _outhit (CallFunction|ShootTrace))
      (if (.bBlockingHit (Collision|BreakHitResult _outhit))
        (Variables|Internal|SetImpactPoint (.ImpactPoint (Collision|BreakHitResult _outhit)))
        (Variables|Internal|SetRot (.rotation (Math|Transform|MakeTransform (Transformation|GetWorldLocation (Variables|/Game/GAME/Core/BP_CoreCharacter.BP_CoreCharacter_C|GetAimArrow (Variables|Refs|GetCharacterRef))) (Math|Rotator|MakeRotfromX (- (.ImpactPoint (Collision|BreakHitResult _outhit)) _returnvalue)))))
        (else
          (Variables|Internal|SetImpactPoint (.TraceEnd (Collision|BreakHitResult _outhit)))
          (Variables|Internal|SetRot (Math|Rotator|MakeRotfromX (- (.TraceEnd (Collision|BreakHitResult _outhit)) _returnvalue)))))
      (bind _output_get (Variables|Internal|SetCurrentImpactPoint (Variables|Internal|GetImpactPoint)))
      (bind _output_get_2 (Variables|Internal|SetCurrentTraceStart (.TraceStart (Collision|BreakHitResult _outhit))))
      (Variables|Internal|SetCurrentTraceRotation (Variables|Internal|GetRot))
      (bind _output_get_3 (Variables|Internal|SetCurrentMuzzleLocation (Transformation|GetSocketLocation (Variables|Default|GetWeaponMesh) "Muzzle")))
      (return _outhit _output_get _output_get_2 (Variables|Internal|GetRot) _output_get_3))
    (:else)))

(fn SprayLineHorizontal
  (params (InVec :type Vector))
  (bind (_x _y _z) (Math|Vector|BreakVector InVec))
  (return (Math|Vector|MakeVector (+ _x 1e+03) (+ _y -1e+03) _z)))

(fn EquiptoPlayer
  (params (Parent :type Scene%20Component%20Object%20Reference))
  (bind _root (Variables|Default|GetRoot))
  (Collision|SetCollisionEnabled _root "NoCollision")
  (Rendering|SetVisibility _root false false)
  (Transformation|AttachComponentToComponent (Variables|Default|GetRoot) Parent "None" "SnapToTarget" "SnapToTarget" "SnapToTarget" true))

(event Custom|ChangeShotgunFiringDirection
  (params (FireCenterPellet? :type Boolean))
  (Utilities|FlowControl|DoOnce false
    (:Completed
      (Variables|Internal|SetInternalShotgunSprayOffset 0.0)
      (Variables|Internal|SetShotgunSprayHalfwaySwitch true)
      (if FireCenterPellet?
        (CallFunction|FinishFiring)))))