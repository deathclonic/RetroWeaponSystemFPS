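; BP_Target is a damageable target with a cube mesh that flashes when hit and is destroyed when its health runs out.
; AnyDamage subtracts from Health, then briefly swaps the cube to a hit material before restoring the basic shape material.
; A Damaging flag ignores further damage during the flash and stays set on a lethal hit until the actor is destroyed.
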(event Game|Damage|EventAnyDamage
  (params (Damage :type Float%20%28single-precision%29) (DamageType :type Damage%20Type%20Object%20Reference) (InstigatedBy :type Controller%20Object%20Reference) (DamageCauser :type Actor%20Object%20Reference))
  (if (not (Variables|Default|GetDamaging?))
    (Variables|Default|SetDamaging? true)
    (bind _output_get (Variables|Default|SetHealth (- (stale _output_get) Damage)))
    (if (<= _output_get 0.0)
      (Rendering|Material|SetMaterial (Variables|Default|GetCube) 0 "/Game/GAME/Assets/Materials/MI_Hit.MI_Hit")
      (Utilities|FlowControl|Delay 0.05)
      (Rendering|Material|SetMaterial (Variables|Default|GetCube) 0 "/Engine/BasicShapes/BasicShapeMaterial.BasicShapeMaterial")
      (Utilities|FlowControl|Delay 0.025)
      (Actor|DestroyActor)
      (else
        (Rendering|Material|SetMaterial (Variables|Default|GetCube) 0 "/Game/GAME/Assets/Materials/MI_Hit.MI_Hit")
        (Utilities|FlowControl|Delay 0.05)
        (Rendering|Material|SetMaterial (Variables|Default|GetCube) 0 "/Engine/BasicShapes/BasicShapeMaterial.BasicShapeMaterial")
        (Variables|Default|SetDamaging? false)))))

(fn ConstructionScript)